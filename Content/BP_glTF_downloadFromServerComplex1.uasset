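; Actor that downloads a glTF file from a URL on BeginPlay and builds its meshes at runtime using glTFRuntime.
; The download goes to memory, printing progress and status, then the data is parsed and each node becomes a new static mesh component.
; Nodes get complex-as-simple collision with nav collision, except those named "Door", which load with the default mesh config through GenerateWithoutCollision.
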(event `self.ReceiveBeginPlay`
  ;[1 0.3483 0.7722] Start Here
  (`FileToMemoryDownloader.DownloadFileToMemory` (`self.URL`) 0.0 "" false (`|CreateDelegate` :!event `Progress`) (`|CreateDelegate` :!event `DownloadDone`)))

(event `Progress`
  (params (BytesReceived :type Integer64) (ContentLength :type Integer64) (ProgressRatio :type "Float (single-precision)"))
  ;[1 1 1] Progress
  (`KismetSystemLibrary.PrintString` (`KismetTextLibrary.Conv_TextToString` (`|FormatText` "glTF_Download: {bytes}/{total}" BytesReceived ContentLength)) true true (struct :`G` 0.66 :`B` 1.0 :`A` 1.0) 100.0))

(event `DownloadDone`
  (params (DownloadedContent :type "Array of Byte (by ref)") (Result :type "EDownloadToMemoryResult Enum" :default "Success"))
  ;[1 1 1] Downloaded
  (`KismetSystemLibrary.PrintString` (`KismetTextLibrary.Conv_TextToString` (`|FormatText` "glTF_D/L Status: {status}" (`|GetEnumeratorNameAsString` Result))) true true (struct :`G` 0.66 :`B` 1.0 :`A` 1.0) 100.0)
  (bind _returnvalue (`glTFRuntimeFunctionLibrary.glTFLoadAssetFromData` DownloadedContent))
  (for _array_element (`glTFRuntimeAsset.GetNodes` _returnvalue)
    (bind (_index _name _transform _meshindex) (break `glTFRuntimeNode` _array_element))
    (switch `string` _name
      (:`Default`
        (`self.GenerateWithCollision` _returnvalue _meshindex))
      (:`Door`
        (`self.GenerateWithoutCollision` _returnvalue _meshindex)))))

(fn `GenerateWithCollision`
  (params (glTFObjectRef :type "glTFRuntimeAsset Object Reference") (meshIndex :type Integer))
  (bind _returnvalue (`AddComponent|NODE_AddStaticMeshComponent-1`))
  (bind _returnvalue_2 (`glTFRuntimeAsset.LoadStaticMesh` glTFObjectRef meshIndex (make `glTFRuntimeStaticMeshConfig` :`bBuildComplexCollision` true :`CollisionComplexity` "CTF_UseComplexAsSimple" :`bAllowCPUAccess` true :`Outer` _returnvalue :`bBuildNavCollision` true)))
  (`StaticMeshComponent.SetStaticMesh` _returnvalue _returnvalue_2))

(fn `GenerateWithoutCollision`
  (params (glTFObjectRef :type "glTFRuntimeAsset Object Reference") (meshIndex :type Integer))
  (bind _returnvalue (`AddComponent|NODE_AddStaticMeshComponent-0`))
  (bind _returnvalue_2 (`glTFRuntimeAsset.LoadStaticMesh` :`self` glTFObjectRef :`MeshIndex` meshIndex))
  (`StaticMeshComponent.SetStaticMesh` _returnvalue _returnvalue_2))

(fn `UserConstructionScript`)