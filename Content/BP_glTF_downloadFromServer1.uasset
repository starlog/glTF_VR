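; Actor that downloads a glTF model from a URL at BeginPlay and spawns it into the level at runtime.
; It downloads to memory, printing byte progress and the final status, then loads the data through the glTFRuntime plugin.
; The result spawns as a glTFRuntimeAssetActor at this actor's transform, using complex-as-simple collision, CPU access and nav collision.
; The completion handler does not check the download result before loading.
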(event `self.ReceiveBeginPlay`
  ;[1 0.3483 0.7722] Start Here
  (`FileToMemoryDownloader.DownloadFileToMemory` (`self.URL`) 0.0 "" false (`|CreateDelegate` :!event `Progress`) (`|CreateDelegate` :!event `DownloadDone`)))

(event `Progress`
  (params (BytesReceived :type Integer64) (ContentLength :type Integer64) (ProgressRatio :type "Float (single-precision)"))
  ;[1 1 1] Progress
  (`KismetSystemLibrary.PrintString` (`KismetTextLibrary.Conv_TextToString` (`|FormatText` "glTF_Download: {bytes}/{total}" BytesReceived ContentLength)) true true (struct :`G` 0.66 :`B` 1.0 :`A` 1.0) 100.0))

(event `DownloadDone`
  (params (DownloadedContent :type "Array of Byte (by ref)") (Result :type "EDownloadToMemoryResult Enum" :default "Success"))
  ;[0.4548 0.5799 1] Download Complete
  (`KismetSystemLibrary.PrintString` (`KismetTextLibrary.Conv_TextToString` (`|FormatText` "glTF_D/L Status: {status}" (`|GetEnumeratorNameAsString` Result))) true true (struct :`G` 0.66 :`B` 1.0 :`A` 1.0) 100.0)
  (bind _returnvalue (`glTFRuntimeFunctionLibrary.glTFLoadAssetFromData` DownloadedContent))
  (`|SpawnActorFromClass` "/Script/glTFRuntime.glTFRuntimeAssetActor" (`self.GetTransform`) "Undefined" "MultiplyWithRoot" null _returnvalue (make `glTFRuntimeStaticMeshConfig` :`bBuildSimpleCollision` false :`bBuildComplexCollision` true :`CollisionComplexity` "CTF_UseComplexAsSimple" :`bAllowCPUAccess` true :`Outer` (`self.DefaultSceneRoot`) :`bBuildNavCollision` true) (struct) (struct) (struct) true false true true true true false -1 false true null))

(fn `UserConstructionScript`)